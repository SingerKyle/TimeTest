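; Four-tumbler combination lock puzzle, driven by keys that select a tumbler and spin it forward or back.
; Timelines animate the selected tumbler's roll from one shared rotation value, with DoOnce gates blocking repeat spins mid-animation.
; Each press also derives that tumbler's digit from its current roll, without awaiting the animation, then compares the joined digits to Combination.
; A match triggers nothing yet, and RandomizeTumbler, affecting only the first tumbler, is never called here.
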(event `Key|Down`
  (params (Key :type "Key Structure"))
  (:`Pressed`
    (`self.SpinTmbler` :!label _label)
    (`self.Number Set`)
    (`self.CheckCombination`)))

(event `Key|NumPadTwo`
  (params (Key :type "Key Structure"))
  (:`Pressed`
    (goto _label)))

(event `Key|Up`
  (params (Key :type "Key Structure"))
  (:`Pressed`
    (`self.SpinTumBack` :!label _label_2)
    (`self.Number Set`)
    (`self.CheckCombination`)))

(event `Key|Right`
  (params (Key :type "Key Structure"))
  (:`Pressed`
    (if (== (`self.TumblerMesh1`) (`self.CurrentTumbler`))
      _
      (elif (== (`self.CurrentTumbler`) (`self.TumblerMesh4`))
        (set `self.CurrentTumbler` (`self.TumblerMesh3`))
        (elif (== (`self.TumblerMesh3`) (`self.CurrentTumbler`))
          (set `self.CurrentTumbler` (`self.TumblerMesh2`))
          (elif (== (`self.CurrentTumbler`) (`self.TumblerMesh2`))
            (set `self.CurrentTumbler` (`self.TumblerMesh1`))))))))

(event `Key|NumPadEight`
  (params (Key :type "Key Structure"))
  (:`Pressed`
    (goto _label_2)))

(event `Key|Four`
  (params (Key :type "Key Structure"))
  (:`Pressed`
    (if (== (`self.CurrentTumbler`) (`self.TumblerMesh4`)) :!label _label_3
      _
      (elif (== (`self.CurrentTumbler`) (`self.TumblerMesh1`))
        (set `self.CurrentTumbler` (`self.TumblerMesh2`))
        (elif (== (`self.CurrentTumbler`) (`self.TumblerMesh2`))
          (set `self.CurrentTumbler` (`self.TumblerMesh3`))
          (elif (== (`self.CurrentTumbler`) (`self.TumblerMesh3`))
            (set `self.CurrentTumbler` (`self.TumblerMesh4`))))))))

(event `Key|Left`
  (params (Key :type "Key Structure"))
  (:`Pressed`
    (goto _label_3)))

(event `CheckCombination`
  (if (`KismetStringLibrary.EqualEqual_StrStr` (`KismetStringLibrary.Concat_StrStr` (`KismetStringLibrary.Conv_IntToString` (`self.TumblerNumber1`)) (`KismetStringLibrary.Conv_IntToString` (`self.TumblerNumber2`)) (`KismetStringLibrary.Conv_IntToString` (`self.TumblerNumber3`)) (`KismetStringLibrary.Conv_IntToString` (`self.TumblerNumber4`))) (`self.Combination`))
    _))

(event `self.ReceiveBeginPlay`
  (set `self.CurrentTumbler` (`self.TumblerMesh1`)))

(event `SpinTmbler`
  ;[1 1 1] Spin Tumbler
  (`/Engine/EditorBlueprintResources/StandardMacros.DoOnce` false :!label _label_4
    (:`Completed`
      (bind (_direction _alpha) (`Timeline|Timeline` :!via `PlayFromStart`)
        (:`Update`
          (bind _returnvalue (+ (`self.TumblerRotation`) _alpha))
          (`SceneComponent.K2_SetRelativeRotation` (`self.CurrentTumbler`) (`KismetMathLibrary.MakeRotator` _returnvalue) false false))
        (:`Finished`
          (set `self.TumblerRotation` _returnvalue)
          (`self.SpinTumblerReset`)
          (if (>= (`self.TumblerRotation`) 360.0)
            (set `self.TumblerRotation` 0.0)))))))

(event `SpinTumblerReset`
  ;[1 1 1] Spin Tumbler
  (goto _label_4 :!via `Reset`))

(event `SpinTumBack`
  ;[1 1 1] Spin Tumbler
  (`/Engine/EditorBlueprintResources/StandardMacros.DoOnce` false :!label _label_5
    (:`Completed`
      (bind (_direction _alpha) (`Timeline|Timeline_0` :!via `PlayFromStart`)
        (:`Update`
          (bind _returnvalue (- (`self.TumblerRotation`) _alpha))
          (`SceneComponent.K2_SetRelativeRotation` (`self.CurrentTumbler`) (`KismetMathLibrary.MakeRotator` _returnvalue) false false))
        (:`Finished`
          (set `self.TumblerRotation` _returnvalue)
          (`self.SpinTumBackReset`)
          (if (<= (`self.TumblerRotation`) -360.0)
            (set `self.TumblerRotation` 0.0)))))))

(event `SpinTumBackReset`
  ;[1 1 1] Spin Tumbler
  (goto _label_5 :!via `Reset`))

(fn `Number Set`
  (bind _relativerotation_roll (`KismetMathLibrary.BreakRotator` (`SceneComponent.RelativeRotation` (`self.TumblerMesh4`))))
  (bind _relativerotation_roll_2 (`KismetMathLibrary.BreakRotator` (`SceneComponent.RelativeRotation` (`self.TumblerMesh1`))))
  (bind _relativerotation_roll_3 (`KismetMathLibrary.BreakRotator` (`SceneComponent.RelativeRotation` (`self.TumblerMesh2`))))
  (bind _relativerotation_roll_4 (`KismetMathLibrary.BreakRotator` (`SceneComponent.RelativeRotation` (`self.TumblerMesh3`))))
  (if (== (`self.CurrentTumbler`) (`self.TumblerMesh1`))
    (set `self.TumblerNumber1` (`KismetMathLibrary.FTrunc` (/ (`KismetMathLibrary.Abs` _relativerotation_roll_2) 36.0)))
    (elif (== (`self.CurrentTumbler`) (`self.TumblerMesh2`))
      (set `self.TumblerNumber2` (`KismetMathLibrary.FTrunc` (/ (`KismetMathLibrary.Abs` _relativerotation_roll_3) 36.0)))
      (elif (== (`self.CurrentTumbler`) (`self.TumblerMesh3`))
        (set `self.TumblerNumber3` (`KismetMathLibrary.FTrunc` (/ (`KismetMathLibrary.Abs` _relativerotation_roll_4) 36.0)))
        (elif (== (`self.CurrentTumbler`) (`self.TumblerMesh4`))
          (set `self.TumblerNumber4` (`KismetMathLibrary.FTrunc` (/ (`KismetMathLibrary.Abs` _relativerotation_roll) 36.0))))))))

(fn `RandomizeTumbler`
  (bind _randomrotations (`self.RandomRotations`))
  (bind _output_get (set `self.TumblerRotation` (`|GetArrayItem` _randomrotations (`KismetMathLibrary.RandomIntegerInRange` 0 (- (`KismetArrayLibrary.Array_Length` _randomrotations) 1)))))
  (`SceneComponent.K2_SetRelativeRotation` (`self.TumblerMesh1`) (`KismetMathLibrary.MakeRotator` _output_get) false false))

(fn `UserConstructionScript`)