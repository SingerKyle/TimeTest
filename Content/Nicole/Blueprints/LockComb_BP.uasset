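; Combination lock actor that unlocks when the four digits on its child tumbler actor match the Comb string.
; Tick and UnlockStuff feed a one-second delayed check; the first match clears LockedState and briefly simulates physics on the lock mesh.
; BeginPlay optionally randomizes the tumblers.
; A configurable trigger volume toggles UsingLock on the overlapping first-person character.
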(event `self.ReceiveTick`
  (params (DeltaSeconds :type "Float (single-precision)"))
  (bind _lockmesh (`self.LockMesh`))
  ;[1 1 1] check for correct combination
  (`KismetSystemLibrary.Delay` 1.0 :!label _label)
  (bind _combomatch_ (`self.CheckComb`))
  (if _combomatch_
    (`/Engine/EditorBlueprintResources/StandardMacros.DoOnce` false
      (:`Completed`
        (set `self.LockedState` false)
        (`KismetSystemLibrary.Delay` 1.5)
        (`SkeletalMeshComponent.SetAllBodiesSimulatePhysics` _lockmesh true)
        (`KismetSystemLibrary.Delay` 0.4)
        (`KismetSystemLibrary.Delay` 2.0)
        (`SkeletalMeshComponent.SetAllBodiesSimulatePhysics` _lockmesh false)))))

(event `UnlockStuff`
  ;[1 1 1] check for correct combination
  (goto _label))

(event `self.ReceiveBeginPlay`
  ;[1 1 1] randomize tumblers?
  (if (`self.RandomTumRot?`)
    (`/Game/Nicole/Blueprints/LockTumbler_BP.RandomizeTumbler` (cast `/Game/Nicole/Blueprints/LockTumbler_BP` (`ChildActorComponent.ChildActor` (`self.LockTumbler1_BP`)) :!pure true))))

(event `self.LockTrigger.OnComponentBeginOverlap`
  (params (OverlappedComponent :type "PrimitiveComponent Object Reference") (OtherActor :type "Actor Object Reference") (OtherComp :type "PrimitiveComponent Object Reference") (OtherBodyIndex :type Integer) (bFromSweep :type Boolean) (SweepResult :type "HitResult Structure (by ref)"))
  (bind _asbp_first_person_character (cast `/Game/FirstPerson/Blueprints/BP_FirstPersonCharacter` OtherActor))
  (set `/Game/FirstPerson/Blueprints/BP_FirstPersonCharacter.UsingLock` true _asbp_first_person_character))

(event `self.LockTrigger.OnComponentEndOverlap`
  (params (OverlappedComponent :type "PrimitiveComponent Object Reference") (OtherActor :type "Actor Object Reference") (OtherComp :type "PrimitiveComponent Object Reference") (OtherBodyIndex :type Integer))
  (bind _asbp_first_person_character (cast `/Game/FirstPerson/Blueprints/BP_FirstPersonCharacter` OtherActor))
  (set `/Game/FirstPerson/Blueprints/BP_FirstPersonCharacter.UsingLock` false _asbp_first_person_character))

(fn `CheckComb`
  (returns (`ComboMatch?` :type Boolean))
  (bind _aslock_tumbler_bp (cast `/Game/Nicole/Blueprints/LockTumbler_BP` (`ChildActorComponent.ChildActor` (`self.LockTumbler1_BP`)) :!pure true))
  (return (`KismetStringLibrary.EqualEqual_StrStr` (`self.Comb`) (`KismetStringLibrary.Concat_StrStr` (`KismetStringLibrary.Conv_IntToString` (`/Game/Nicole/Blueprints/LockTumbler_BP.TumblerNumber1` _aslock_tumbler_bp)) (`KismetStringLibrary.Conv_IntToString` (`/Game/Nicole/Blueprints/LockTumbler_BP.TumblerNumber2` _aslock_tumbler_bp)) (`KismetStringLibrary.Conv_IntToString` (`/Game/Nicole/Blueprints/LockTumbler_BP.TumblerNumber3` _aslock_tumbler_bp)) (`KismetStringLibrary.Conv_IntToString` (`/Game/Nicole/Blueprints/LockTumbler_BP.TumblerNumber4` _aslock_tumbler_bp))))))

(fn `UserConstructionScript`
  (bind _locktrigger (`self.LockTrigger`))
  (`SceneComponent.SetRelativeScale3D` _locktrigger (`self.LockTriggerScale`))
  (`SceneComponent.K2_SetRelativeLocation` _locktrigger (`self.LockTrigLoc`) false false))