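; SwitchPuzzle_BP is a code-entry puzzle where the first-person character overlaps switches in sequence to trigger a linked light.
; The construction script spawns a spaced row of meshes and trigger boxes, one per CorrectCode character, tagging each box with a StartCode character.
; Overlaps append that tag to InputCode, which, at full length, either calls SwitchLightMessage on the Light if correct or clears if wrong.
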(fn `AddCode`
  (params (Add :type String))
  (set `self.InputCode` (`KismetStringLibrary.Concat_StrStr` (`self.InputCode`) Add))
  (if (== (`KismetStringLibrary.Len` (`self.CorrectCode`)) (`KismetStringLibrary.Len` (`self.InputCode`)))
    (if (== (`self.CorrectCode`) (`self.InputCode`))
      (`KismetSystemLibrary.LogString` "worked")
      (message `/Game/4-Blueprints/Puzzles/Puzzle_IN.SwitchLight` (`self.Light`))
      (else
        (`KismetSystemLibrary.LogString` "failed")
        (set `self.InputCode` "")))))

(fn `SwitchPuzzle_BP_AutoGenFunc`
  (params (OverlappedComponent :type "PrimitiveComponent Object Reference") (OtherActor :type "Actor Object Reference") (OtherComp :type "PrimitiveComponent Object Reference") (OtherBodyIndex :type Integer) (bFromSweep :type Boolean) (SweepResult :type "HitResult Structure (by ref)"))
  (cast `/Game/FirstPerson/Blueprints/BP_FirstPersonCharacter` OtherActor
    (:`then`
      (`self.AddCode` (`KismetStringLibrary.Conv_NameToString` (`|GetArrayItem` (`ActorComponent.ComponentTags` OverlappedComponent))))
      (return))
    (:`CastFailed`
      (`KismetSystemLibrary.PrintString` "cast is failing"))))

(fn `UserConstructionScript`
  (for _index (range (`KismetStringLibrary.Len` (`self.CorrectCode`)))
    (bind _returnvalue (`AddComponent|NODE_AddStaticMeshComponent-0` :`RelativeTransform` (`KismetMathLibrary.MakeTransform` (`KismetMathLibrary.MakeVector` (* _index (`self.spacing`))))))
    (bind _returnvalue_2 (`AddComponent|NODE_AddBoxComponent-0` :`RelativeTransform` (`KismetMathLibrary.MakeTransform` (+ (`SceneComponent.RelativeLocation` _returnvalue) (0.0 40.0 -20.0)) (struct) (0.2 1.0 3.0))))
    (set `ActorComponent.ComponentTags` (`|MakeArray` (`KismetStringLibrary.Conv_StringToName` (`KismetStringLibrary.GetSubstring` (`self.StartCode`) _index))) _returnvalue_2)
    (add `PrimitiveComponent.OnComponentBeginOverlap` _returnvalue_2 (`|CreateDelegate` :!event `SwitchPuzzle_BP_AutoGenFunc`))))