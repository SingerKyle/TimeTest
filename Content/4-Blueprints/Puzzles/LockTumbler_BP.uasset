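; Four-tumbler combination lock puzzle, controlled by keyboard while flagged as being viewed.
; Left/Right select a tumbler highlighted through custom depth, Up/Down spin it with timelines and sound, and R resets all.
; After each spin, NumberIncrease derives the digit from mesh roll in 36-degree steps, snapping some angles.
; CheckCombination compares the concatenated digits to Combination, but a match only clears the highlight.
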(event `Key|BackSpace`
  (params (Key :type "Key Structure")))

(event `SetViewed`
  (set `self.IsBeingViewed?` true))

(event `SetNotViewed`
  (set `self.IsBeingViewed?` false))

(event `DisableRenderTarget`
  (`PrimitiveComponent.SetRenderCustomDepth` (`self.CurrentTumbler`) false))

(event `Key|R`
  (params (Key :type "Key Structure"))
  ;[1 1 1] Reset tumblers
  (:`Pressed`
    (if (`self.IsBeingViewed?`)
      (`SceneComponent.K2_SetRelativeRotation` :`self` (`self.TumblerMesh1`))
      (`SceneComponent.K2_SetRelativeRotation` :`self` (`self.TumblerMesh4`))
      (`SceneComponent.K2_SetRelativeRotation` :`self` (`self.TumblerMesh3`))
      (`SceneComponent.K2_SetRelativeRotation` :`self` (`self.TumblerMesh2`))
      (set `self.TumblerNumber1` 0)
      (set `self.TumblerNumber2` 0)
      (set `self.TumblerNumber4` 0)
      (set `self.TumblerNumber3` 0)
      (`PrimitiveComponent.SetRenderCustomDepth` (`self.CurrentTumbler`) false)
      (bind _output_get (set `self.CurrentTumbler` (`self.TumblerMesh4`)))
      (`PrimitiveComponent.SetRenderCustomDepth` _output_get true))))

(event `self.ReceiveTick`
  (params (DeltaSeconds :type "Float (single-precision)")))

(event `SpinTmbler`
  (bind _tumblerrotation (`self.TumblerRotation`))
  (bind _relativerotation_roll (`KismetMathLibrary.BreakRotator` (`SceneComponent.RelativeRotation` (`self.CurrentTumbler`))))
  ;[1 1 1] Spin Tumbler
  (set `self.CanRotate` false)
  (set `self.TumblerRotation` _relativerotation_roll)
  (`/Engine/EditorBlueprintResources/StandardMacros.DoOnce` false :!label _label
    (:`Completed`
      (bind (_direction _alpha) (`Timeline|Timeline` :!via `PlayFromStart`)
        (:`Update`
          (bind _returnvalue (+ (`self.TumblerRotation`) _alpha))
          (`SceneComponent.K2_SetRelativeRotation` (`self.CurrentTumbler`) (`KismetMathLibrary.MakeRotator` _returnvalue) false false))
        (:`Finished`
          (set `self.TumblerRotation` _returnvalue)
          (`self.SpinTumblerReset`)
          (if (>= _tumblerrotation 360.0)
            (set `self.TumblerRotation` 0.0)
            (elif (< _tumblerrotation 0.0)
              (set `self.TumblerRotation` (`KismetMathLibrary.Abs` _tumblerrotation)))))))))

(event `Key|Right`
  (params (Key :type "Key Structure"))
  ;[1 1 1] Select the tumbler to the right of the current tumbler
  (:`Pressed`
    (if (`self.IsBeingViewed?`)
      (if (`self.CanRotate`)
        (`PrimitiveComponent.SetRenderCustomDepth` (`self.CurrentTumbler`) false)
        (if (== (`self.TumblerMesh1`) (`self.CurrentTumbler`))
          _
          (elif (== (`self.CurrentTumbler`) (`self.TumblerMesh4`))
            (set `self.CurrentTumbler` (`self.TumblerMesh3`))
            (`KismetSystemLibrary.PrintString` "Selecting Tumbler 3")
            (`PrimitiveComponent.SetRenderCustomDepth` (`self.CurrentTumbler`) true :!label _label_2)
            (elif (== (`self.TumblerMesh3`) (`self.CurrentTumbler`))
              (set `self.CurrentTumbler` (`self.TumblerMesh2`))
              (`KismetSystemLibrary.PrintString` "Selecting Tumbler 2")
              (goto _label_2)
              (elif (== (`self.CurrentTumbler`) (`self.TumblerMesh2`))
                (set `self.CurrentTumbler` (`self.TumblerMesh1`))
                (`KismetSystemLibrary.PrintString` "Selecting Tumbler 1")
                (goto _label_2)))))))))

(event `SpinTumblerReset`
  ;[1 1 1] Spin Tumbler
  (goto _label :!via `Reset`))

(event `SpinTumBack`
  (bind _tumblerrotation (`self.TumblerRotation`))
  (bind _relativerotation_roll (`KismetMathLibrary.BreakRotator` (`SceneComponent.RelativeRotation` (`self.CurrentTumbler`))))
  ;[1 1 1] Spin Tumbler
  (set `self.CanRotate` false)
  (set `self.TumblerRotation` _relativerotation_roll)
  (`/Engine/EditorBlueprintResources/StandardMacros.DoOnce` false :!label _label_3
    (:`Completed`
      (bind (_direction _alpha) (`Timeline|Timeline_0` :!via `PlayFromStart`)
        (:`Update`
          (bind _returnvalue (- (`self.TumblerRotation`) _alpha))
          (`SceneComponent.K2_SetRelativeRotation` (`self.CurrentTumbler`) (`KismetMathLibrary.MakeRotator` _returnvalue) false false))
        (:`Finished`
          (set `self.TumblerRotation` _returnvalue)
          (`self.SpinTumBackReset`)
          (if (<= _tumblerrotation -360.0)
            (set `self.TumblerRotation` 0.0)
            (elif (< _tumblerrotation 0.0)
              (set `self.TumblerRotation` (`KismetMathLibrary.Abs` _tumblerrotation)))))))))

(event `SpinTumBackReset`
  ;[1 1 1] Spin Tumbler
  (goto _label_3 :!via `Reset`))

(event `Key|Left`
  (params (Key :type "Key Structure"))
  ;[1 1 1] Select The tumbler to the left of the current tumbler
  (:`Pressed`
    (if (`self.IsBeingViewed?`)
      (if (`self.CanRotate`)
        (`PrimitiveComponent.SetRenderCustomDepth` (`self.CurrentTumbler`) false)
        (if (== (`self.CurrentTumbler`) (`self.TumblerMesh4`))
          _
          (elif (== (`self.CurrentTumbler`) (`self.TumblerMesh1`))
            (set `self.CurrentTumbler` (`self.TumblerMesh2`))
            (`KismetSystemLibrary.PrintString` "Selecting Tumbler 2")
            (`PrimitiveComponent.SetRenderCustomDepth` (`self.CurrentTumbler`) true :!label _label_4)
            (elif (== (`self.CurrentTumbler`) (`self.TumblerMesh2`))
              (set `self.CurrentTumbler` (`self.TumblerMesh3`))
              (`KismetSystemLibrary.PrintString` "Selecting Tumbler3")
              (goto _label_4)
              (elif (== (`self.CurrentTumbler`) (`self.TumblerMesh3`))
                (set `self.CurrentTumbler` (`self.TumblerMesh4`))
                (`KismetSystemLibrary.PrintString` "Selecting Tumbler4")
                (goto _label_4)))))))))

(event `self.ReceiveBeginPlay`
  ;[1 1 1] Begin Play
  (bind _output_get (set `self.CurrentTumbler` (`self.TumblerMesh4`)))
  (`PrimitiveComponent.SetRenderCustomDepth` _output_get false))

(event `Key|Down`
  (params (Key :type "Key Structure"))
  ;[1 1 1] Rotate the current tumbler down
  (:`Pressed`
    (if (`self.IsBeingViewed?`)
      (`/Engine/EditorBlueprintResources/StandardMacros.DoOnce` false :!label _label_5
        (:`Completed`
          (`PrimitiveComponent.SetRenderCustomDepth` (`self.CurrentTumbler`) true)
          (if (`self.CanRotate`)
            (`GameplayStatics.PlaySound2D` "/Game/2-Audio/SoundEffects/tumblerTurn_Cue.tumblerTurn_Cue" 1.0 1.0 0.0 null null)
            (`self.SpinTmbler`)
            (`KismetSystemLibrary.Delay` 0.7)
            (`self.Number Increase`)
            (`self.CheckCombination`)
            (set `self.CanRotate` true)
            (goto _label_5 :!via `Reset`))))))
  (:`Released`
    (`KismetSystemLibrary.RetriggerableDelay` 0.5)
    (goto _label_5 :!via `Reset`)))

(event `CheckCombination`
  (bind _returnvalue (`KismetStringLibrary.Concat_StrStr` (`KismetStringLibrary.Conv_IntToString` (`self.TumblerNumber4`)) (`KismetStringLibrary.Conv_IntToString` (`self.TumblerNumber3`)) (`KismetStringLibrary.Conv_IntToString` (`self.TumblerNumber2`)) (`KismetStringLibrary.Conv_IntToString` (`self.TumblerNumber1`))))
  ;[1 1 1] Check the input against the code
  (`KismetSystemLibrary.PrintString` _returnvalue)
  (if (`KismetStringLibrary.EqualEqual_StrStr` _returnvalue (`self.Combination`))
    (`PrimitiveComponent.SetRenderCustomDepth` (`self.CurrentTumbler`) false)))

(event `Key|Up`
  (params (Key :type "Key Structure"))
  ;[1 1 1] Rotate the current tumbler up
  (:`Pressed`
    (if (`self.IsBeingViewed?`)
      (`/Engine/EditorBlueprintResources/StandardMacros.DoOnce` false :!label _label_6
        (:`Completed`
          (`PrimitiveComponent.SetRenderCustomDepth` (`self.CurrentTumbler`) true)
          (if (`self.CanRotate`)
            (`GameplayStatics.PlaySound2D` "/Game/2-Audio/SoundEffects/tumblerTurn_Cue.tumblerTurn_Cue" 1.0 1.0 0.0 null null)
            (`self.SpinTumBack`)
            (`KismetSystemLibrary.Delay` 0.7)
            (`self.Number Increase`)
            (`self.CheckCombination`)
            (set `self.CanRotate` true)
            (goto _label_6 :!via `Reset`))))))
  (:`Released`
    (`KismetSystemLibrary.RetriggerableDelay` 0.5)
    (goto _label_6 :!via `Reset`)))

(fn `Number Increase`
  (bind _relativerotation_roll (`KismetMathLibrary.BreakRotator` (`SceneComponent.RelativeRotation` (`self.TumblerMesh4`))))
  (bind _relativerotation_roll_2 (`KismetMathLibrary.BreakRotator` (`SceneComponent.RelativeRotation` (`self.TumblerMesh1`))))
  (bind _relativerotation_roll_3 (`KismetMathLibrary.BreakRotator` (`SceneComponent.RelativeRotation` (`self.TumblerMesh2`))))
  (bind _relativerotation_roll_4 (`KismetMathLibrary.BreakRotator` (`SceneComponent.RelativeRotation` (`self.TumblerMesh3`))))
  (bind _returnvalue (`KismetMathLibrary.FFloor` _relativerotation_roll_2))
  (bind _returnvalue_2 (`KismetMathLibrary.FFloor` _relativerotation_roll_3))
  (bind _returnvalue_3 (`KismetMathLibrary.FFloor` _relativerotation_roll_4))
  (bind _returnvalue_4 (`KismetMathLibrary.FFloor` _relativerotation_roll))
  (bind _returnvalue_5 (`KismetMathLibrary.FTrunc` (`KismetMathLibrary.Abs` _relativerotation_roll_2)))
  (bind _returnvalue_6 (/ (`KismetMathLibrary.Abs` _relativerotation_roll_3) 36.0))
  (bind _returnvalue_7 (`KismetMathLibrary.FTrunc` _returnvalue_6))
  ;[1 1 1] If turning tumbler 1
  (if (== (`self.CurrentTumbler`) (`self.TumblerMesh1`))
    ;[1 1 1] This Checks the rotation value of the current tumbler and returns the value shown on the face
    (if (< _relativerotation_roll_2 0.0)
      (if (or (== _returnvalue 0) (< _returnvalue -144))
        (set `self.TumblerNumber1` 5)
        (`SceneComponent.K2_SetRelativeRotation` (`self.CurrentTumbler`) (struct :`Roll` 180.0) false false)
        (elif (== _returnvalue -144)
          (set `self.TumblerNumber1` 6)
          (`SceneComponent.K2_SetRelativeRotation` (`self.CurrentTumbler`) (struct :`Roll` -144.0) false false)
          (elif (== _returnvalue -108)
            (set `self.TumblerNumber1` 7)
            (`SceneComponent.K2_SetRelativeRotation` (`self.CurrentTumbler`) (struct :`Roll` -108.0) false false)
            (elif (== _returnvalue -72)
              (set `self.TumblerNumber1` 8)
              (`SceneComponent.K2_SetRelativeRotation` (`self.CurrentTumbler`) (struct :`Roll` -72.0) false false)
              (elif (and (> _returnvalue -37) (< _returnvalue -34))
                (set `self.TumblerNumber1` 9)
                (`SceneComponent.K2_SetRelativeRotation` (`self.CurrentTumbler`) (struct :`Roll` -36.0) false false))))))
      (`KismetSystemLibrary.PrintString` (`KismetStringLibrary.Concat_StrStr` "Tumbler 1:" (`KismetStringLibrary.Conv_IntToString` (`KismetMathLibrary.FTrunc` _relativerotation_roll_2))) :!label _label)
      (set `self.CanRotate` true)
      (elif (== _returnvalue_5 36)
        (set `self.TumblerNumber1` _returnvalue_5)
        (`SceneComponent.K2_SetRelativeRotation` (`self.CurrentTumbler`) (struct :`Roll` 36.0) false false)
        (goto _label)
        (elif (== _returnvalue_5 72)
          (set `self.TumblerNumber1` _returnvalue_5)
          (`SceneComponent.K2_SetRelativeRotation` (`self.CurrentTumbler`) (struct :`Roll` 72.0) false false)
          (goto _label)
          (elif (== _returnvalue_5 108)
            (set `self.TumblerNumber1` _returnvalue_5)
            (`SceneComponent.K2_SetRelativeRotation` (`self.CurrentTumbler`) (struct :`Roll` 108.0) false false)
            (goto _label)
            (elif (== _returnvalue_5 144)
              (set `self.TumblerNumber1` _returnvalue_5)
              (`SceneComponent.K2_SetRelativeRotation` (`self.CurrentTumbler`) (struct :`Roll` 144.0) false false)
              (goto _label)
              (elif (== _returnvalue_5 180)
                (set `self.TumblerNumber1` _returnvalue_5)
                (`SceneComponent.K2_SetRelativeRotation` (`self.CurrentTumbler`) (struct :`Roll` 180.0) false false)
                (goto _label)))))))
    (else
      ;[1 1 1] Checks If second tumbler is selected and changes the face number to 1/36 of the rotation value
      ;;[1 1 1] If tumbler is 2
      (if (== (`self.CurrentTumbler`) (`self.TumblerMesh2`))
        ;;[1 1 1] If rotation value is +ve or -ve
        (if (< _relativerotation_roll_3 0.0)
          ;;[1 1 1] if -ve we set the number value manually
          (if (or (== _returnvalue_2 0) (< _returnvalue_2 -144))
            (set `self.TumblerNumber2` 5)
            (`SceneComponent.K2_SetRelativeRotation` (`self.CurrentTumbler`) (struct :`Roll` 180.0) false false)
            (elif (== _returnvalue_2 -144)
              (set `self.TumblerNumber2` 6)
              (`SceneComponent.K2_SetRelativeRotation` (`self.CurrentTumbler`) (struct :`Roll` -144.0) false false)
              (elif (== _returnvalue_2 -108)
                (set `self.TumblerNumber2` 7)
                (`SceneComponent.K2_SetRelativeRotation` (`self.CurrentTumbler`) (struct :`Roll` -108.0) false false)
                (elif (== _returnvalue_2 -72)
                  (set `self.TumblerNumber2` 8)
                  (`SceneComponent.K2_SetRelativeRotation` (`self.CurrentTumbler`) (struct :`Roll` -72.0) false false)
                  (elif (and (> _returnvalue_2 -37) (< _returnvalue_2 -34))
                    (set `self.TumblerNumber2` 9)
                    (`SceneComponent.K2_SetRelativeRotation` (`self.CurrentTumbler`) (struct :`Roll` -36.0) false false))))))
          (elif (== _returnvalue_7 (`self.TumblerNumber2`))
            ;;[1 1 1] if +ve we devide by 36
            (set `self.TumblerNumber2` (`KismetMathLibrary.FCeil` _returnvalue_6))
            (else
              (set `self.TumblerNumber2` _returnvalue_7))))
        ;[1 1 1] print the current tumbler number
        (`KismetSystemLibrary.PrintString` (`KismetStringLibrary.Concat_StrStr` "Tumbler 2:" (`KismetStringLibrary.Conv_IntToString` (`KismetMathLibrary.FTrunc` _relativerotation_roll_3))))
        (set `self.CanRotate` true)
        (else
          ;[1 1 1] 3rd tumbler
          (if (== (`self.CurrentTumbler`) (`self.TumblerMesh3`))
            (if (< _relativerotation_roll_4 0.0)
              (`KismetSystemLibrary.PrintString` (`KismetStringLibrary.Conv_DoubleToString` _relativerotation_roll_4))
              ;;[1 1 1] Manually set
              ;;;[1 1 1] added this
              (if (or (== _returnvalue_3 0) (< _returnvalue_3 -144))
                (set `self.TumblerNumber3` 5)
                (`SceneComponent.K2_SetRelativeRotation` (`self.CurrentTumbler`) (struct :`Roll` 180.0) false false)
                (elif (== _returnvalue_3 -144)
                  (set `self.TumblerNumber3` 6)
                  (`SceneComponent.K2_SetRelativeRotation` (`self.CurrentTumbler`) (struct :`Roll` -144.0) false false)
                  (elif (== _returnvalue_3 -108)
                    (set `self.TumblerNumber3` 7)
                    (`SceneComponent.K2_SetRelativeRotation` (`self.CurrentTumbler`) (struct :`Roll` -108.0) false false)
                    (elif (== _returnvalue_3 -72)
                      (set `self.TumblerNumber3` 8)
                      (`SceneComponent.K2_SetRelativeRotation` (`self.CurrentTumbler`) (struct :`Roll` -72.0) false false)
                      (elif (and (> _returnvalue_3 -37) (< _returnvalue_3 -34))
                        (set `self.TumblerNumber3` 9)
                        (`SceneComponent.K2_SetRelativeRotation` (`self.CurrentTumbler`) (struct :`Roll` -36.0) false false))))))
              (else
                ;;[1 1 1] +ve
                (set `self.TumblerNumber3` (`KismetMathLibrary.FTrunc` (/ (`KismetMathLibrary.Abs` _relativerotation_roll_4) 36.0)))))
            ;[1 1 1] Prints the set  face number
            (`KismetSystemLibrary.PrintString` (`KismetStringLibrary.Concat_StrStr` "Tumbler 3:" (`KismetStringLibrary.Conv_IntToString` (`KismetMathLibrary.FTrunc` _relativerotation_roll_4))))
            (set `self.CanRotate` true)
            (else
              ;[1 1 1] 4th tumbler
              ;;[1 1 1] if 4th tumbler
              (if (== (`self.CurrentTumbler`) (`self.TumblerMesh4`))
                (if (< _relativerotation_roll 0.0)
                  ;;[1 1 1] 6-9, when the value is -ve
                  (if (or (== _returnvalue_4 0) (< _returnvalue_4 -144))
                    (set `self.TumblerNumber4` 5)
                    (`SceneComponent.K2_SetRelativeRotation` (`self.CurrentTumbler`) (struct :`Roll` 180.0) false false)
                    (elif (== _returnvalue_4 -144)
                      (set `self.TumblerNumber4` 6)
                      (`SceneComponent.K2_SetRelativeRotation` (`self.CurrentTumbler`) (struct :`Roll` -144.0) false false)
                      (elif (== _returnvalue_4 -108)
                        (set `self.TumblerNumber4` 7)
                        (`SceneComponent.K2_SetRelativeRotation` (`self.CurrentTumbler`) (struct :`Roll` -108.0) false false)
                        (elif (== _returnvalue_4 -72)
                          (set `self.TumblerNumber4` 8)
                          (`SceneComponent.K2_SetRelativeRotation` (`self.CurrentTumbler`) (struct :`Roll` -72.0) false false)
                          (elif (and (> _returnvalue_4 -37) (< _returnvalue_4 -34))
                            (set `self.TumblerNumber4` 9)
                            (`SceneComponent.K2_SetRelativeRotation` (`self.CurrentTumbler`) (struct :`Roll` -36.0) false false))))))
                  (else
                    ;;[1 1 1] 1-5, is +ve
                    (set `self.TumblerNumber4` (`KismetMathLibrary.FTrunc` (/ (`KismetMathLibrary.Abs` _relativerotation_roll) 36.0)))))
                ;[1 1 1] Prints the face value
                (`KismetSystemLibrary.PrintString` (`KismetStringLibrary.Concat_StrStr` "Tumbler 4:" (`KismetStringLibrary.Conv_IntToString` (`KismetMathLibrary.FTrunc` _relativerotation_roll))))
                (set `self.CanRotate` true)
                (else
                  (`KismetSystemLibrary.PrintString` "Something has gone very wrong"))))))))))

(fn `RandomizeTumbler`
  (bind _randomrotations (`self.RandomRotations`))
  (bind _output_get (set `self.TumblerRotation` (`|GetArrayItem` _randomrotations (`KismetMathLibrary.RandomIntegerInRange` 0 (- (`KismetArrayLibrary.Array_Length` _randomrotations) 1)))))
  (`SceneComponent.K2_SetRelativeRotation` (`self.TumblerMesh1`) (`KismetMathLibrary.MakeRotator` _output_get) false false))

(fn `UserConstructionScript`)