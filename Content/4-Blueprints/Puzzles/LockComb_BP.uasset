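; Four-digit combination padlock puzzle that unlocks a door for the first-person character.
; A LockTumbler child actor holds the four digits, optionally randomized at BeginPlay, and receives view and highlight calls.
; While locked, Tick compares the concatenated digits to Comb, then once plays sounds, briefly simulates lock physics and clears the player's DoorIsLocked.
; A construction-configured trigger sets the player's UsingLock flag on overlap.
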(event `SetNotViewing`
  (bind _aslock_tumbler_bp (cast `/Game/4-Blueprints/Puzzles/LockTumbler_BP` (`ChildActorComponent.ChildActor` (`self.LockTumbler1_BP`))))
  (`/Game/4-Blueprints/Puzzles/LockTumbler_BP.SetViewed` _aslock_tumbler_bp))

(event `SetViewing`
  (bind _aslock_tumbler_bp (cast `/Game/4-Blueprints/Puzzles/LockTumbler_BP` (`ChildActorComponent.ChildActor` (`self.LockTumbler1_BP`))))
  (`/Game/4-Blueprints/Puzzles/LockTumbler_BP.SetViewed` _aslock_tumbler_bp))

(event `DisableHighlight#`
  (bind _aslock_tumbler_bp (cast `/Game/4-Blueprints/Puzzles/LockTumbler_BP` (`ChildActorComponent.ChildActor` (`self.LockTumbler1_BP`))))
  (`/Game/4-Blueprints/Puzzles/LockTumbler_BP.DisableRenderTarget` _aslock_tumbler_bp))

(event `self.ReceiveTick`
  (params (DeltaSeconds :type "Float (single-precision)"))
  (bind _lockmesh (`self.LockMesh`))
  ;[1 1 1] check for correct combination
  (if (`self.IsLocked?`)
    (bind _combomatch_ (`self.CheckComb` :!label _label))
    (if _combomatch_
      (`/Engine/EditorBlueprintResources/StandardMacros.DoOnce` false
        (:`Completed`
          (`GameplayStatics.PlaySound2D` "/Game/2-Audio/Padlock.Padlock" 1.0 1.0 0.0 null null)
          (set `self.IsDoorLocked?` false)
          (`KismetSystemLibrary.Delay` 1.5)
          (`SkeletalMeshComponent.SetAllBodiesSimulatePhysics` _lockmesh true)
          (`GameplayStatics.PlaySound2D` "/Game/2-Audio/ChainSound.ChainSound" 1.0 1.0 0.0 null null)
          (`KismetSystemLibrary.Delay` 0.4)
          (`KismetSystemLibrary.Delay` 2.0)
          (`SkeletalMeshComponent.SetAllBodiesSimulatePhysics` _lockmesh false)
          (bind _asbp_first_person_character (cast `/Game/FirstPerson/Blueprints/BP_FirstPersonCharacter` (`GameplayStatics.GetPlayerCharacter` 0)))
          (set `/Game/FirstPerson/Blueprints/BP_FirstPersonCharacter.DoorIsLocked` (`self.IsDoorLocked?`) _asbp_first_person_character)
          (set `self.IsLocked?` false)
          (`SceneComponent.SetVisibility` (`self.LockTumbler1_BP`) false false))))))

(event `UnlockStuff`
  ;[1 1 1] check for correct combination
  (goto _label))

(event `self.ReceiveBeginPlay`
  ;[1 1 1] randomize tumblers?
  (if (`self.RandomTumRot?`)
    (`/Game/4-Blueprints/Puzzles/LockTumbler_BP.RandomizeTumbler` (cast `/Game/4-Blueprints/Puzzles/LockTumbler_BP` (`ChildActorComponent.ChildActor` (`self.LockTumbler1_BP`)) :!pure true))))

(event `self.LockTrigger.OnComponentBeginOverlap`
  (params (OverlappedComponent :type "PrimitiveComponent Object Reference") (OtherActor :type "Actor Object Reference") (OtherComp :type "PrimitiveComponent Object Reference") (OtherBodyIndex :type Integer) (bFromSweep :type Boolean) (SweepResult :type "HitResult Structure (by ref)"))
  (bind _asbp_first_person_character (cast `/Game/FirstPerson/Blueprints/BP_FirstPersonCharacter` OtherActor))
  (set `/Game/FirstPerson/Blueprints/BP_FirstPersonCharacter.UsingLock` true _asbp_first_person_character))

(event `self.LockTrigger.OnComponentEndOverlap`
  (params (OverlappedComponent :type "PrimitiveComponent Object Reference") (OtherActor :type "Actor Object Reference") (OtherComp :type "PrimitiveComponent Object Reference") (OtherBodyIndex :type Integer))
  (bind _asbp_first_person_character (cast `/Game/FirstPerson/Blueprints/BP_FirstPersonCharacter` OtherActor))
  (set `/Game/FirstPerson/Blueprints/BP_FirstPersonCharacter.UsingLock` false _asbp_first_person_character))

(fn `CheckComb`
  (returns (`ComboMatch?` :type Boolean))
  (bind _aslock_tumbler_bp (cast `/Game/4-Blueprints/Puzzles/LockTumbler_BP` (`ChildActorComponent.ChildActor` (`self.LockTumbler1_BP`)) :!pure true))
  (return (`KismetStringLibrary.EqualEqual_StrStr` (`self.Comb`) (`KismetStringLibrary.Concat_StrStr` (`KismetStringLibrary.Conv_IntToString` (`/Game/4-Blueprints/Puzzles/LockTumbler_BP.TumblerNumber1` _aslock_tumbler_bp)) (`KismetStringLibrary.Conv_IntToString` (`/Game/4-Blueprints/Puzzles/LockTumbler_BP.TumblerNumber2` _aslock_tumbler_bp)) (`KismetStringLibrary.Conv_IntToString` (`/Game/4-Blueprints/Puzzles/LockTumbler_BP.TumblerNumber3` _aslock_tumbler_bp)) (`KismetStringLibrary.Conv_IntToString` (`/Game/4-Blueprints/Puzzles/LockTumbler_BP.TumblerNumber4` _aslock_tumbler_bp))))))

(fn `UserConstructionScript`
  (bind _locktrigger (`self.LockTrigger`))
  (`SceneComponent.SetRelativeScale3D` _locktrigger (`self.LockTriggerScale`))
  (`SceneComponent.K2_SetRelativeLocation` _locktrigger (`self.LockTrigLoc`) false false))