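; Newspaper puzzle Blueprint that reveals or hides a plane once enough items are collected.
; CollectItem increments a counter, and DisplayCheck compares it to the maximum.
; When the count reaches the maximum, a DoOnce gate calls DisplayImage once to toggle the plane's visibility.
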(event `DIsplay Image`
  (`SceneComponent.ToggleVisibility` (`self.Plane`) false))

(event `Collect Item`
  (`/Engine/EditorBlueprintResources/StandardMacros.IncrementInt` (`self.currentItems`)))

(event `Display Check`
  (if (>= (`self.currentItems`) (`self.maxItems`))
    (`/Engine/EditorBlueprintResources/StandardMacros.DoOnce` false
      (:`Completed`
        (`self.DIsplay Image`)))))

(fn `UserConstructionScript`)