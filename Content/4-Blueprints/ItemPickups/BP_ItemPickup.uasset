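; BP_ItemPickup is a note pickup that the player collects by walking into its Box trigger.
; On overlap with BP_FirstPersonCharacter, it sets Item1Collected on the character's PlayerInventory and destroys itself.
; The same chain then opens the WB_Note1 widget, switches to Game and UI input with a visible cursor, and plays a paper sound.
; The inventory flag and widget class are hardcoded, so the Blueprint serves only this first item.
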(event `self.ReceiveTick`
  (params (DeltaSeconds :type "Float (single-precision)")))

(event `self.Box.OnComponentBeginOverlap`
  (params (OverlappedComponent :type "PrimitiveComponent Object Reference") (OtherActor :type "Actor Object Reference") (OtherComp :type "PrimitiveComponent Object Reference") (OtherBodyIndex :type Integer) (bFromSweep :type Boolean) (SweepResult :type "HitResult Structure (by ref)"))
  (bind _returnvalue (`GameplayStatics.GetPlayerController` 0))
  (bind _asbp_first_person_character (cast `/Game/FirstPerson/Blueprints/BP_FirstPersonCharacter` OtherActor))
  (set `/Game/4-Blueprints/WidgetBlueprints/WB_Inventory.Item1Collected?` true (`/Game/FirstPerson/Blueprints/BP_FirstPersonCharacter.PlayerInventory` _asbp_first_person_character))
  (`self.K2_DestroyActor`)
  (bind _returnvalue_2 (`|CreateWidget` "/Game/4-Blueprints/WidgetBlueprints/WB_Note1.WB_Note1_C"))
  (bind _output_get (set `self.Widget` _returnvalue_2))
  (`UserWidget.AddToViewport` _output_get 0)
  (`WidgetBlueprintLibrary.SetInputMode_GameAndUIEx` _returnvalue _output_get "DoNotLock" false)
  (set `PlayerController.bShowMouseCursor` true _returnvalue)
  (`GameplayStatics.PlaySound2D` "/Game/2-Audio/SoundEffects/paper_Cue.paper_Cue" 1.0 1.0 0.0 null null))

(fn `UserConstructionScript`)