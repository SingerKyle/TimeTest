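; Interactive door Blueprint that selects its sound according to whether the door is locked, closed or open.
; A custom OpenManually event calls Interact to trigger the door.
; Tick sets the PlaySound variable to the locked sound through a DoOnce, or to the opening or closing sound based on Closed.
; Delay nodes follow the opening and closing assignments, with nothing wired after them.
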(event `OpenManually`
  (`InteractionInterface.Interact` self))

(event `self.ReceiveTick`
  (params (DeltaSeconds :type "Float (single-precision)"))
  (if (`self.locked`)
    (`/Engine/EditorBlueprintResources/StandardMacros.DoOnce` false
      (:`Completed`
        (set `self.PlaySound` "/Game/2-Audio/SoundEffects/lock1.lock1")))
    (elif (`self.closed`)
      (set `self.PlaySound` "/Game/2-Audio/DooropenFinal.DooropenFinal")
      (`KismetSystemLibrary.Delay` 2.0)
      (else
        (set `self.PlaySound` "/Game/2-Audio/doorclosingFinal.doorclosingFinal")
        (`KismetSystemLibrary.Delay` 2.0)))))

(fn `UserConstructionScript`)