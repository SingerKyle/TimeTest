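; Haunted chair scare: a one-shot prop that drags itself away when something overlaps its trigger box.
; The overlap plays a wood-drag sound and a timeline that moves and pitches the mesh, with the track feeding Lerp A and constants feeding Alpha.
; On finish, physics toggles on and back off after a zero delay, then a thump plays.
; An AddImpulse node is left unconnected.
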(event `self.Box.OnComponentBeginOverlap`
  (params (OverlappedComponent :type "PrimitiveComponent Object Reference") (OtherActor :type "Actor Object Reference") (OtherComp :type "PrimitiveComponent Object Reference") (OtherBodyIndex :type Integer) (bFromSweep :type Boolean) (SweepResult :type "HitResult Structure (by ref)"))
  (bind _staticmesh (`self.StaticMesh`))
  (`/Engine/EditorBlueprintResources/StandardMacros.DoOnce` false
    (:`Completed`
      (`GameplayStatics.PlaySoundAtLocation` "/Game/2-Audio/SoundEffects/FastWoodDrag.FastWoodDrag" (`self.K2_GetActorLocation` self) (struct) 1.0 1.0 0.0 null null null null)
      (bind (_direction _newtrack_0) (`Timeline|ChairMove`)
        (:`Update`
          (`SceneComponent.K2_SetRelativeLocationAndRotation` _staticmesh (`KismetMathLibrary.MakeVector` (`KismetMathLibrary.Lerp` _newtrack_0 0.0 1200.0) 0.0 (`KismetMathLibrary.Lerp` _newtrack_0 0.0 -100.0)) (`KismetMathLibrary.MakeRotator` 0.0 (`KismetMathLibrary.Lerp` _newtrack_0 0.0 -90.0)) false false))
        (:`Finished`
          (`PrimitiveComponent.SetSimulatePhysics` _staticmesh true)
          (`KismetSystemLibrary.Delay` 0.0)
          (`PrimitiveComponent.SetSimulatePhysics` (`self.StaticMesh`) false)
          (`GameplayStatics.PlaySoundAtLocation` "/Game/2-Audio/SoundEffects/woodthump2.woodthump2" (`self.K2_GetActorLocation` self) (struct) 1.0 1.0 0.0 null null null null))))))

(fn `UserConstructionScript`)