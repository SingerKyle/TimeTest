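; Scripted door scare that knocks and then swings open a referenced interactive door as the player crosses trigger volumes.
; Entering the playroom trigger arms the Knock volume, which plays two pairs of hit sounds with a dust effect, then enables the Open volume.
; Open, or OtherSide independently, sends the door an interact message once, then hides a weeping angel after a short delay.
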(event `self.OtherSide.OnComponentBeginOverlap`
  (params (OverlappedComponent :type "PrimitiveComponent Object Reference") (OtherActor :type "Actor Object Reference") (OtherComp :type "PrimitiveComponent Object Reference") (OtherBodyIndex :type Integer) (bFromSweep :type Boolean) (SweepResult :type "HitResult Structure (by ref)"))
  (cast `/Game/FirstPerson/Blueprints/BP_FirstPersonCharacter` OtherActor)
  (if (not (`self.DoorOpen?`))
    (`/Engine/EditorBlueprintResources/StandardMacros.DoOnce` false
      (:`Completed`
        (message `InteractionInterface.Interact` (`self.BP_InteractiveDoor`) :!label _label)
        (`/Engine/EditorBlueprintResources/StandardMacros.DoOnce` false
          (:`Completed`
            (set `self.DoorOpen?` true)
            (`KismetSystemLibrary.Delay` 1.0)
            (`SceneComponent.SetVisibility` (`self.WeepingAngel1`) false false)))))))

(event `self.Open.OnComponentBeginOverlap`
  (params (OverlappedComponent :type "PrimitiveComponent Object Reference") (OtherActor :type "Actor Object Reference") (OtherComp :type "PrimitiveComponent Object Reference") (OtherBodyIndex :type Integer) (bFromSweep :type Boolean) (SweepResult :type "HitResult Structure (by ref)"))
  (cast `/Game/FirstPerson/Blueprints/BP_FirstPersonCharacter` OtherActor)
  (if (`self.PlayRoom?`)
    (if (`self.SoundsPlayed?`)
      (goto _label))))

(event `self.Knock.OnComponentBeginOverlap`
  (params (OverlappedComponent :type "PrimitiveComponent Object Reference") (OtherActor :type "Actor Object Reference") (OtherComp :type "PrimitiveComponent Object Reference") (OtherBodyIndex :type Integer) (bFromSweep :type Boolean) (SweepResult :type "HitResult Structure (by ref)"))
  (cast `/Game/FirstPerson/Blueprints/BP_FirstPersonCharacter` OtherActor)
  (if (`self.PlayRoom?`)
    (if (not (`self.DoorOpen?`))
      (`/Engine/EditorBlueprintResources/StandardMacros.DoOnce` false
        (:`Completed`
          (`GameplayStatics.PlaySound2D` "/Game/2-Audio/SoundEffects/doorhit-98828.doorhit-98828" 1.0 1.0 0.0 null null)
          (`SceneComponent.SetVisibility` (`self.DustAttmept2`) true false)
          (`KismetSystemLibrary.Delay` 0.2)
          (`GameplayStatics.PlaySound2D` "/Game/2-Audio/SoundEffects/doorhit-98828.doorhit-98828" 1.0 1.0 0.0 null null)
          (`KismetSystemLibrary.Delay` 1.0)
          (`GameplayStatics.PlaySound2D` "/Game/2-Audio/SoundEffects/doorhit-98828.doorhit-98828" 1.0 1.0 0.0 null null)
          (`KismetSystemLibrary.Delay` 0.2)
          (`GameplayStatics.PlaySound2D` "/Game/2-Audio/SoundEffects/doorhit-98828.doorhit-98828" 1.0 1.0 0.0 null null)
          (set `self.SoundsPlayed?` true)
          (`SceneComponent.SetVisibility` (`self.DustAttmept2`) false false))))))

(event `self.Trigger.OnComponentBeginOverlap`
  (params (OverlappedComponent :type "PrimitiveComponent Object Reference") (OtherActor :type "Actor Object Reference") (OtherComp :type "PrimitiveComponent Object Reference") (OtherBodyIndex :type Integer) (bFromSweep :type Boolean) (SweepResult :type "HitResult Structure (by ref)"))
  (set `self.PlayRoom?` true)
  (`KismetSystemLibrary.PrintString` "been in playroom"))

(fn `UserConstructionScript`)