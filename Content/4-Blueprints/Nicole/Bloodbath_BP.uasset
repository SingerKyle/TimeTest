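; Bloodbath_BP is a one-shot trigger that plays a tap-water sound and animates a sphere, apparently rising blood.
; The first box overlap starts the sound and reveals the sphere, before any player check.
; If the overlapper is the first-person character, the Blood timeline drives the sphere's height and flattened scale.
; A delay called from the timeline update later stops the spawned 2D sound; a separate positioned playback is never stopped.
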(event `self.Box.OnComponentBeginOverlap`
  (params (OverlappedComponent :type "PrimitiveComponent Object Reference") (OtherActor :type "Actor Object Reference") (OtherComp :type "PrimitiveComponent Object Reference") (OtherBodyIndex :type Integer) (bFromSweep :type Boolean) (SweepResult :type "HitResult Structure (by ref)"))
  (`/Engine/EditorBlueprintResources/StandardMacros.DoOnce` false
    (:`Completed`
      (bind _returnvalue (`GameplayStatics.SpawnSound2D` "/Game/2-Audio/SoundEffects/tapwater2_Cue.tapwater2_Cue" 1.0 1.0 0.0 null))
      (`GameplayStatics.PlaySoundAtLocation` (`AudioComponent.Sound` _returnvalue) (8699.837877 -210.801517 413.600444) (struct) 1.0 1.0 0.0 null null null null)
      (`SceneComponent.SetVisibility` (`self.Sphere`) true false)
      (cast `/Game/FirstPerson/Blueprints/BP_FirstPersonCharacter` OtherActor)
      (bind (_direction _alpha) (`Timeline|Blood`)
        (:`Update`
          (`SceneComponent.K2_SetRelativeLocation` (`self.Sphere`) (`KismetMathLibrary.MakeVector` 0.0 0.0 (`KismetMathLibrary.Lerp` _alpha 0.0 -30.0)) false false)
          (`SceneComponent.SetRelativeScale3D` (`self.Sphere`) (`KismetMathLibrary.MakeVector` (`KismetMathLibrary.Lerp` _alpha 0.0 3.6) (`KismetMathLibrary.Lerp` _alpha 0.0 2.12)))
          (`KismetSystemLibrary.Delay` 30.0)
          (if (`AudioComponent.IsPlaying` _returnvalue)
            (`AudioComponent.Stop` _returnvalue)))))))

(fn `UserConstructionScript`)