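; Bookcase actor that topples once, the first time the first-person player overlaps its Box trigger.
; The Fall timeline drives the roll of both bookcase meshes through a Lerp that takes the timeline value as A and a constant as Alpha.
; A one-shot impact sound plays shortly into the fall.
; When the timeline finishes, StaticMesh briefly simulates physics, then stops.
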(event `self.Box.OnComponentBeginOverlap`
  (params (OverlappedComponent :type "PrimitiveComponent Object Reference") (OtherActor :type "Actor Object Reference") (OtherComp :type "PrimitiveComponent Object Reference") (OtherBodyIndex :type Integer) (bFromSweep :type Boolean) (SweepResult :type "HitResult Structure (by ref)"))
  (bind _staticmesh (`self.StaticMesh`))
  (cast `/Game/FirstPerson/Blueprints/BP_FirstPersonCharacter` OtherActor)
  (`/Engine/EditorBlueprintResources/StandardMacros.DoOnce` false
    (:`Completed`
      (bind (_direction _alpha) (`Timeline|Fall`)
        (:`Update`
          (bind _returnvalue (`KismetMathLibrary.Lerp` _alpha 0.0 -22.0))
          (`SceneComponent.K2_SetRelativeRotation` (`self.BookCase`) (`KismetMathLibrary.MakeRotator` _returnvalue) false false)
          (`SceneComponent.K2_SetRelativeRotation` (`self.BookCase1`) (`KismetMathLibrary.MakeRotator` _returnvalue) false false)
          (`KismetSystemLibrary.Delay` 0.45)
          (`/Engine/EditorBlueprintResources/StandardMacros.DoOnce` false
            (:`Completed`
              (`GameplayStatics.PlaySound2D` "/Game/2-Audio/SoundEffects/doorhit-98828.doorhit-98828" 1.0 1.0 0.0 null null))))
        (:`Finished`
          (`PrimitiveComponent.SetSimulatePhysics` _staticmesh true)
          (`KismetSystemLibrary.Delay` 0.55)
          (`PrimitiveComponent.SetSimulatePhysics` _staticmesh false))))))

(fn `UserConstructionScript`)