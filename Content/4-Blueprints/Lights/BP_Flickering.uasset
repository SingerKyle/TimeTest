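; BP_Flickering is a light prop that flickers while the first-person character is inside its Box trigger.
; Character overlap sets PlayerIsClose and starts a Delay-driven loop swapping one static mesh material slot between blue emissive and broken glass in an uneven rhythm.
; Any actor's end overlap clears the flag, which is checked only between passes, so the current pass finishes and leaves the broken glass material.
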(event `self.ReceiveTick`
  (params (DeltaSeconds :type "Float (single-precision)")))

(event `self.Box.OnComponentBeginOverlap`
  (params (OverlappedComponent :type "PrimitiveComponent Object Reference") (OtherActor :type "Actor Object Reference") (OtherComp :type "PrimitiveComponent Object Reference") (OtherBodyIndex :type Integer) (bFromSweep :type Boolean) (SweepResult :type "HitResult Structure (by ref)"))
  (bind _staticmesh (`self.StaticMesh`))
  (bind _staticmesh_2 (`self.StaticMesh`))
  (bind _staticmesh_3 (`self.StaticMesh`))
  (cast `/Game/FirstPerson/Blueprints/BP_FirstPersonCharacter` OtherActor)
  (bind _output_get (set `self.PlayerIsClose` true))
  (if _output_get :!label _label
    (`PrimitiveComponent.SetMaterial` _staticmesh_2 2 "/Game/7-Materials/Emissives/M_BlueEmissive.M_BlueEmissive")
    (`KismetSystemLibrary.Delay` 0.4)
    (`PrimitiveComponent.SetMaterial` _staticmesh_2 2 "/Game/7-Materials/InHouseMaterials/Materials/M_BrokenGlass1.M_BrokenGlass1")
    (`KismetSystemLibrary.Delay` 0.5)
    (`PrimitiveComponent.SetMaterial` _staticmesh_3 2 "/Game/7-Materials/Emissives/M_BlueEmissive.M_BlueEmissive")
    (`KismetSystemLibrary.Delay` 0.1)
    (`PrimitiveComponent.SetMaterial` _staticmesh_3 2 "/Game/7-Materials/InHouseMaterials/Materials/M_BrokenGlass1.M_BrokenGlass1")
    (`KismetSystemLibrary.Delay` 0.5)
    (`PrimitiveComponent.SetMaterial` _staticmesh 2 "/Game/7-Materials/Emissives/M_BlueEmissive.M_BlueEmissive")
    (`KismetSystemLibrary.Delay` 0.1)
    (`PrimitiveComponent.SetMaterial` _staticmesh 2 "/Game/7-Materials/InHouseMaterials/Materials/M_BrokenGlass1.M_BrokenGlass1")
    (goto _label)))

(event `self.Box.OnComponentEndOverlap`
  (params (OverlappedComponent :type "PrimitiveComponent Object Reference") (OtherActor :type "Actor Object Reference") (OtherComp :type "PrimitiveComponent Object Reference") (OtherBodyIndex :type Integer))
  (set `self.PlayerIsClose` false))

(fn `UserConstructionScript`)