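; BP_CaneraStaticTrigger is a trigger volume that occasionally causes a camera static effect on the first-person player.
; When the player overlaps its Box, it checks that Item4 has been collected in the player's inventory, then rolls a one-in-ten chance.
; On success, it calls CameraStatic on the character and stops it after a short randomized delay.
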(event `self.Box.OnComponentBeginOverlap`
  (params (OverlappedComponent :type "PrimitiveComponent Object Reference") (OtherActor :type "Actor Object Reference") (OtherComp :type "PrimitiveComponent Object Reference") (OtherBodyIndex :type Integer) (bFromSweep :type Boolean) (SweepResult :type "HitResult Structure (by ref)"))
  (bind _asbp_first_person_character (cast `/Game/FirstPerson/Blueprints/BP_FirstPersonCharacter` OtherActor))
  (if (`/Game/4-Blueprints/WidgetBlueprints/WB_Inventory.Item4Collected?` (`/Game/FirstPerson/Blueprints/BP_FirstPersonCharacter.PlayerInventory` _asbp_first_person_character))
    (if (== (`KismetMathLibrary.RandomInteger` 10) 0)
      (`/Game/FirstPerson/Blueprints/BP_FirstPersonCharacter.CameraStatic` _asbp_first_person_character)
      (`KismetSystemLibrary.Delay` (`KismetMathLibrary.RandomFloatInRange` 1.5 3.0))
      (`/Game/FirstPerson/Blueprints/BP_FirstPersonCharacter.StopCameraStatic` _asbp_first_person_character))))

(fn `UserConstructionScript`)