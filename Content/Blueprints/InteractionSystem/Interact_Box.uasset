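; Interact_Box is an interactable object that opens a UI widget when interacted with.
; Its InteractwithObject event prints a debug message, then creates an Interact_Widget for the first player controller and adds it to the viewport.
; It then shows the mouse cursor and switches input to UI only, with focus on the new widget.
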(event `self.InteractWithObject`
  (bind _returnvalue (`GameplayStatics.GetPlayerController` 0))
  (`KismetSystemLibrary.PrintString` "You touched me")
  (bind _returnvalue_2 (`|CreateWidget` "/Game/Blueprints/InteractionSystem/Interact_Widget.Interact_Widget_C" _returnvalue))
  (`UserWidget.AddToViewport` _returnvalue_2 0)
  (set `PlayerController.bShowMouseCursor` true _returnvalue)
  (`WidgetBlueprintLibrary.SetInputMode_UIOnlyEx` _returnvalue _returnvalue_2))

(fn `UserConstructionScript`
  (`parent.UserConstructionScript`))