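; Interactable door actor that plays a dialogue clip with a subtitle and sends the player to the Hotel level.
; InteractwithObject prints a debug string, plays SoundClip at the mesh, shows SubtitleText through a WB_Subtitle widget, then immediately calls OpenLevelByName with no delay.
; A separate CreateDisplayWidget event opens an Interact_Widget with mouse cursor and UI-only input, and GetName returns the Name variable.
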(event `CreateDisplayWidget`
  (bind _returnvalue (`GameplayStatics.GetPlayerController` 0))
  (bind _returnvalue_2 (`|CreateWidget` "/Game/Blueprints/InteractionSystem/Interact_Widget.Interact_Widget_C" _returnvalue))
  (`UserWidget.AddToViewport` _returnvalue_2 0)
  (set `PlayerController.bShowMouseCursor` true _returnvalue)
  (`WidgetBlueprintLibrary.SetInputMode_UIOnlyEx` _returnvalue _returnvalue_2))

(event `CreateSubtitle`
  (params (TextToShow :type Text))
  (bind _returnvalue (`|CreateWidget` "/Game/Blueprints/InteractionSystem/WB_Subtitle.WB_Subtitle_C" (`GameplayStatics.GetPlayerController` 0)))
  (bind _output_get (set `self.Subtitle` _returnvalue))
  (bind _aswb_subtitle (cast `/Game/Blueprints/InteractionSystem/WB_Subtitle` _output_get))
  (set `/Game/Blueprints/InteractionSystem/WB_Subtitle.TextToDisplay` TextToShow _aswb_subtitle)
  (`UserWidget.AddToViewport` _returnvalue 0))

(event `self.InteractWithObject`
  (`KismetSystemLibrary.PrintString` "You touched me")
  (`GameplayStatics.PlaySoundAtLocation` (`self.SoundClip`) (`SceneComponent.K2_GetComponentLocation` (`self.StaticMesh`)) (struct) 1.0 1.0 0.0 null null null null)
  (`self.CreateSubtitle` (`self.SubtitleText`))
  (`GameplayStatics.OpenLevel` "Hotel"))

(fn `Get Name`
  (returns (Name :type Text))
  (return (`self.Name`)))

(fn `UserConstructionScript`
  (`parent.UserConstructionScript`))